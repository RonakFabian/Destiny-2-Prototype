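; Behavior Tree task that selects the next patrol waypoint for an AI-controlled pawn.
; It reads the PatrolPoints array from the pawn cast to ThirdPersonCharacter, then writes the point at the Blackboard Index to the WayPoint key.
; It then increments Index, wrapping by array length so the route loops, and finishes successfully.
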(event `self.ReceiveExecuteAI`
  (params (OwnerController :type "AIController Object Reference") (ControlledPawn :type "Pawn Object Reference"))
  (`self.GetPatrolPoints` ControlledPawn)
  (bind _index (`self.SetPatrolPoint`))
  (`self.CycleIndex` _index)
  (`self.FinishExecute` true))

(fn `CycleIndex`
  (params (Index :type Integer))
  (`BTFunctionLibrary.SetBlackboardValueAsInt` (`self.Index`) (mod (+ Index 1) (`KismetArrayLibrary.Array_Length` (`self.PatrolPoints`)))))

(fn `GetPatrolPoints`
  (params (Object :type "Object Object Reference"))
  (bind _asthird_person_character (cast `/Game/ThirdPersonCPP/Blueprints/ThirdPersonCharacter` Object))
  (set `self.PatrolPoints` (`/Game/ThirdPersonCPP/Blueprints/ThirdPersonCharacter.Patrol Points` _asthird_person_character)))

(fn `SetPatrolPoint`
  (returns (index :type Integer))
  (bind _returnvalue (`BTFunctionLibrary.GetBlackboardValueAsInt` (`self.Index`)))
  (`BTFunctionLibrary.SetBlackboardValueAsObject` (`self.WayPoint`) (`|GetArrayItem` (`self.PatrolPoints`) _returnvalue))
  (return _returnvalue))