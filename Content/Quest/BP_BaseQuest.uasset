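; BP_BaseQuest is a base quest Blueprint that tracks progress toward a required amount in a QuestData struct.
; UpdateCount increments the current amount while the quest is incomplete and sets the completed flag when it equals the required amount.
; Each update prints either the new count or a completion message on screen.
; CheckIfCompleted is an empty stub.
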(fn `CheckIfCompleted`)

(fn `UpdateCount`
  (bind _questdata (`self.QuestData`))
  (bind (_iscompleted _questname _questdescription _currentamount _requiredamount) (break `/Game/Quest/QuestData` _questdata))
  (if (not _iscompleted)
    (bind _result (`/Engine/EditorBlueprintResources/StandardMacros.IncrementInt` _currentamount)
      (:`  `
        (if (== _currentamount _requiredamount)
          (`KismetSystemLibrary.PrintString` null "Completed" true true (struct :`R` 1.0 :`B` 0.258956 :`A` 1.0))
          (setmembers `/Game/Quest/QuestData` :`StructRef` _questdata :`isCompleted` true)
          (else
            (setmembers `/Game/Quest/QuestData` :`StructRef` _questdata :`currentAmount` _result)
            (`KismetSystemLibrary.PrintString` null (`KismetStringLibrary.Conv_IntToString` _result) true true (struct :`R` 1.0 :`B` 0.258956 :`A` 1.0))))))))