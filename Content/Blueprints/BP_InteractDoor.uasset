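; Hold-to-open double door that acts as a mission step, built on a parent that appears to supply the mission logic.
; While it can execute and the overlap box is occupied, Tick polls the E key's hold time and feeds progress to BP_D2HUD, scaled by a fixed divisor rather than HoldTimer.
; Reaching HoldTimer disables it, swings both meshes oppositely via timeline, removes the waypoint widget and triggers the next mission event.
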(event `self.Box.OnComponentBeginOverlap`
  (params (OverlappedComponent :type "PrimitiveComponent Object Reference") (OtherActor :type "Actor Object Reference") (OtherComp :type "PrimitiveComponent Object Reference") (OtherBodyIndex :type Integer) (bFromSweep :type Boolean) (SweepResult :type "HitResult Structure (by ref)"))
  (set `self.isInTrigger` true)
  (if (`self.canExecute`)
    (cast `/Game/FirstPersonCPP/Blueprints/FirstPersonCharacter` OtherActor)
    (`KismetSystemLibrary.PrintString` (`KismetStringLibrary.Concat_StrStr` "Player Entered " (`KismetSystemLibrary.GetObjectName` self)))))

(event `self.ReceiveTick`
  (params (DeltaSeconds :type "Float (single-precision)"))
  (bind _returnvalue (`PlayerController.GetInputKeyTimeDown` (`GameplayStatics.GetPlayerController` 0) "E"))
  (`parent.ReceiveTick` DeltaSeconds)
  (if (`self.canExecute`)
    (if (`self.isInTrigger`)
      (set `/Game/Blueprints/BP_D2HUD.Progress` (/ _returnvalue 2.0) (`self.NewVar_0`))
      (if (>= _returnvalue (`self.HoldTimer`))
        (`KismetSystemLibrary.PrintString` "DoorOpened")
        (set `self.canExecute` false)
        (`self.OpenDoor`)
        (`Widget.RemoveFromParent` (`self.WayPointWidget`))
        (set `/Game/Blueprints/BP_D2HUD.Progress` 0.0 (`self.NewVar_0`))
        (`/Game/Quest/MissionEventHelper.ExecuteNextMissionEvent`)))))

(event `OpenDoor`
  ;[1 1 1] Door Rotation
  (bind (_direction _newtrack_0) (`Timeline|Timeline_0` :!via `PlayFromStart`)
    (:`Update`
      (`SceneComponent.K2_SetRelativeRotation` (`self.StaticMesh1`) (`KismetMathLibrary.MakeRotator` 0.0 0.0 (* -1 _newtrack_0)) false false)
      (`SceneComponent.K2_SetRelativeRotation` (`self.StaticMesh`) (`KismetMathLibrary.MakeRotator` 0.0 0.0 _newtrack_0) false false))))

(event `self.Box.OnComponentEndOverlap`
  (params (OverlappedComponent :type "PrimitiveComponent Object Reference") (OtherActor :type "Actor Object Reference") (OtherComp :type "PrimitiveComponent Object Reference") (OtherBodyIndex :type Integer))
  (set `self.isInTrigger` false)
  (set `self.currentTimer` 0.0))

(event `self.ReceiveBeginPlay`
  (`parent.ReceiveBeginPlay`)
  (bind _asbp_d2hud (cast `/Game/Blueprints/BP_D2HUD` (`PlayerController.GetHUD` (`GameplayStatics.GetPlayerController` 0))))
  (set `/Game/Blueprints/BP_D2HUD.Progress` (`self.MyProgress`) _asbp_d2hud)
  (set `self.NewVar_0` _asbp_d2hud))

(fn `UserConstructionScript`
  (`parent.UserConstructionScript`))