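; Base enemy actor that tracks health and dies when it runs out.
; BeginPlay sets CurrentHealth to MaxHealth, and TakeDamage subtracts the given amount, triggering death at zero or below.
; EnemyDeath broadcasts the OnEnemyDeath dispatcher with a fixed enemy type and itself, then destroys the actor.
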(event `self.ReceiveBeginPlay`
  (set `self.currentHealth` (`self.maxHealth`)))

(fn `Enemy Death`
  (`self.OnEnemyDeath` "NewEnumerator1" self)
  (`self.K2_DestroyActor`))

(fn `TakeDamage`
  (params (DmgAmount :type Integer))
  (set `self.currentHealth` (- (`self.currentHealth`) DmgAmount))
  (if (<= (`self.currentHealth`) 0)
    (`self.Enemy Death`)))

(fn `UserConstructionScript`)