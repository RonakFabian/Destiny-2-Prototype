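; Interactable chest that serves as a mission step, completed by holding the E key for a set time.
; While it can execute, Tick polls how long E is held, then disables the chest, removes its waypoint widget and fires the next mission event.
; Box overlaps track whether something is in the trigger and print player entry, but the hold check ignores that flag, so the key works from anywhere.
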(event `self.Box.OnComponentBeginOverlap`
  (params (OverlappedComponent :type "PrimitiveComponent Object Reference") (OtherActor :type "Actor Object Reference") (OtherComp :type "PrimitiveComponent Object Reference") (OtherBodyIndex :type Integer) (bFromSweep :type Boolean) (SweepResult :type "HitResult Structure (by ref)"))
  (set `self.isInTrigger` true)
  (if (`self.canExecute`)
    (cast `/Game/FirstPersonCPP/Blueprints/FirstPersonCharacter` OtherActor)
    (`KismetSystemLibrary.PrintString` (`KismetStringLibrary.Concat_StrStr` "Player Entered " (`KismetSystemLibrary.GetObjectName` self)))))

(event `self.ReceiveTick`
  (params (DeltaSeconds :type "Float (single-precision)"))
  (`parent.ReceiveTick` DeltaSeconds)
  (if (`self.canExecute`)
    (if (>= (`PlayerController.GetInputKeyTimeDown` (`GameplayStatics.GetPlayerController` 0) "E") (`self.HoldTimer`))
      (`KismetSystemLibrary.PrintString` "Done")
      (set `self.canExecute` false)
      (`Widget.RemoveFromParent` (`self.WayPointWidget`))
      (`/Game/Quest/MissionEventHelper.ExecuteNextMissionEvent`))))

(event `self.Box.OnComponentEndOverlap`
  (params (OverlappedComponent :type "PrimitiveComponent Object Reference") (OtherActor :type "Actor Object Reference") (OtherComp :type "PrimitiveComponent Object Reference") (OtherBodyIndex :type Integer))
  (set `self.isInTrigger` false)
  (set `self.currentTimer` 0.0))

(fn `UserConstructionScript`
  (`parent.UserConstructionScript`))