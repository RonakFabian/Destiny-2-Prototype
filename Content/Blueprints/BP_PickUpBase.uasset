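; Base pickup actor that the first-person character can collect into the HUD inventory and later use to boost Health, Energy and Mood.
; Its sphere shows or hides a pickup-text widget and tracks whether the character is in range.
; The character's OnPickUpItem dispatcher adds its item struct, holding a self-reference, to the inventory, then hides the actor instead of destroying it.
; UseAction applies the stat bonuses and destroys it; DropAction is empty.
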(event `self.ReceiveBeginPlay`
  (bind _pickuptextref (`self.PickUpTextRef`))
  (bind (_item _thumbnail _pickuptext _actiontext) (break `/Game/Blueprints/InventoryStruct` (`self.ItemInfo`)))
  (bind _returnvalue (`|CreateWidget` "/Game/UMG/PIckupText.PIckupText_C" (`GameplayStatics.GetPlayerController` 0)))
  (bind _output_get (set `self.PickUpTextRef` _returnvalue))
  (bind _structout (setmembers `/Game/Blueprints/InventoryStruct` :`StructRef` (make `/Game/Blueprints/InventoryStruct` self _thumbnail _pickuptext _actiontext)))
  (set `self.ItemInfo` _structout)
  (set `/Game/UMG/PIckupText.PickUpActor` self _pickuptextref)
  (set `/Game/UMG/PIckupText.PickupText` _pickuptext _pickuptextref)
  (bind _asfirst_person_character (cast `/Game/FirstPersonCPP/Blueprints/FirstPersonCharacter` (`GameplayStatics.GetPlayerPawn` 0)))
  (bind _output_get_2 (set `self.CharacterRef` _asfirst_person_character))
  (add `/Game/FirstPersonCPP/Blueprints/FirstPersonCharacter.OnPickUpItem` _output_get_2 (delegate `OnPickUpItem`)))

(event `OnPickUpItem`
  (bind _gamehudref (`/Game/FirstPersonCPP/Blueprints/FirstPersonCharacter.GameHUDRef` (`self.CharacterRef`)))
  (if (and (`self.GetActorEnableCollision`) (`self.IsInRange`))
    (`KismetArrayLibrary.Array_Add` (`/Game/UMG/GameHUD.Inventory` _gamehudref) (`self.ItemInfo`))
    (`Widget.RemoveFromParent` (`self.PickUpTextRef`))
    (`self.SetActorHiddenInGame` true)
    (`self.SetActorEnableCollision` false)
    (`/Game/UMG/GameHUD.RefreshInventory` _gamehudref)))

(event `self.Sphere.OnComponentBeginOverlap`
  (params (OverlappedComponent :type "PrimitiveComponent Object Reference") (OtherActor :type "Actor Object Reference") (OtherComp :type "PrimitiveComponent Object Reference") (OtherBodyIndex :type Integer) (bFromSweep :type Boolean) (SweepResult :type "HitResult Structure (by ref)"))
  (cast `/Game/FirstPersonCPP/Blueprints/FirstPersonCharacter` OtherActor)
  (`UserWidget.AddToViewport` (`self.PickUpTextRef`) 0)
  (set `self.IsInRange` true)
  (`KismetSystemLibrary.PrintString` "Hello"))

(event `self.Sphere.OnComponentEndOverlap`
  (params (OverlappedComponent :type "PrimitiveComponent Object Reference") (OtherActor :type "Actor Object Reference") (OtherComp :type "PrimitiveComponent Object Reference") (OtherBodyIndex :type Integer))
  (cast `/Game/FirstPersonCPP/Blueprints/FirstPersonCharacter` OtherActor)
  (`Widget.RemoveFromParent` (`self.PickUpTextRef`))
  (set `self.IsInRange` false))

(event `/Game/UMG/ActionInterface.UseAction`
  (bind _characterref (`self.CharacterRef`))
  ;[1 1 1] Use Item
  (set `/Game/FirstPersonCPP/Blueprints/FirstPersonCharacter.Health` (+ (`/Game/FirstPersonCPP/Blueprints/FirstPersonCharacter.Health` _characterref) (`self.AddHealth`)) _characterref)
  (set `/Game/FirstPersonCPP/Blueprints/FirstPersonCharacter.Energy` (+ (`/Game/FirstPersonCPP/Blueprints/FirstPersonCharacter.Energy` _characterref) (`self.AddEnergy`)) _characterref)
  (set `/Game/FirstPersonCPP/Blueprints/FirstPersonCharacter.Mood` (+ (`/Game/FirstPersonCPP/Blueprints/FirstPersonCharacter.Mood` _characterref) (`self.AddMood`)) _characterref)
  (`self.K2_DestroyActor`))

(event `/Game/UMG/ActionInterface.DropAction`
  (params (ItemToDrop :type "Actor Object Reference")))

(fn `UserConstructionScript`)