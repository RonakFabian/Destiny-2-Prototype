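; A trigger-volume mission step that completes when the first-person player character enters its box.
; On BeginPlay it creates a WayPoint widget owned by this actor.
; When the mission event begins, it arms the trigger after a short delay and shows the waypoint.
; A valid overlap while armed disarms it, starts the next mission event and removes the waypoint.
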(event `self.ReceiveBeginPlay`
  (`parent.ReceiveBeginPlay`)
  (bind _returnvalue (`|CreateWidget` "/Game/UMG/WayPoint.WayPoint_C" (`GameplayStatics.GetPlayerController` 0)))
  (bind _output_get (set `self.WayPointWidget` _returnvalue))
  (set `/Game/UMG/WayPoint.OwningActor` self _output_get)
  (`self.EnableInput` (`GameplayStatics.GetPlayerController` 0)))

(event `self.Box.OnComponentBeginOverlap`
  (params (OverlappedComponent :type "PrimitiveComponent Object Reference") (OtherActor :type "Actor Object Reference") (OtherComp :type "PrimitiveComponent Object Reference") (OtherBodyIndex :type Integer) (bFromSweep :type Boolean) (SweepResult :type "HitResult Structure (by ref)"))
  (if (`self.canExecute`)
    (cast `/Game/FirstPersonCPP/Blueprints/FirstPersonCharacter` OtherActor)
    (`KismetSystemLibrary.PrintString` (`KismetStringLibrary.Concat_StrStr` "Player Entered " (`KismetSystemLibrary.GetObjectName` self)))
    (set `self.canExecute` false)
    (`/Game/Quest/MissionEventHelper.ExecuteNextMissionEvent`)
    (`Widget.RemoveFromParent` (`self.WayPointWidget`))))

(event `self.BeginExecuteMissionEvent`
  (`KismetSystemLibrary.Delay` 0.2)
  (set `self.canExecute` true)
  (`KismetSystemLibrary.PrintString` "Started")
  (`UserWidget.AddToViewport` (`self.WayPointWidget`) 0))

(fn `UserConstructionScript`
  (`parent.UserConstructionScript`))