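; BP_MyPatrollingGuard is a guard actor that bobs its mesh and can be killed by damage; it contains no patrol movement logic.
; While CanMove is set, Tick offsets the mesh's relative Z by a time-based sine, accumulating each frame without delta-time scaling.
; A custom TakeDamage function subtracts from CurrentHealth, then at zero or below spawns an enlarged bullet-impact particle effect and destroys the actor.
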(event `self.ReceiveTick`
  (params (DeltaSeconds :type "Float (single-precision)"))
  (if (`self.canMove`)
    (`SceneComponent.K2_SetRelativeLocation` (`self.Mesh`) (`KismetMathLibrary.MakeVector` 0.0 0.0 (+ (.z (.location (`SceneComponent.GetRelativeTransform` (`self.Mesh`)))) (* (`KismetMathLibrary.Sin` (* (`GameplayStatics.GetTimeSeconds`) 10.0)) 1.0))) false false)))

(fn `TakeDamage`
  (params (NewParam :type Integer))
  (bind (_returnvalue_location _returnvalue_rotation) (`KismetMathLibrary.BreakTransform` (`self.GetTransform`)))
  (set `self.Current Health` (- (`self.Current Health`) NewParam))
  (if (<= (`self.Current Health`) 0)
    (`GameplayStatics.SpawnEmitterAtLocation` "/Game/Effects/ParticleSystems/Gameplay/Player/P_body_bullet_impact.P_body_bullet_impact" _returnvalue_location _returnvalue_rotation (10.0 10.0 10.0) true "AutoRelease")
    (`self.K2_DestroyActor`)))

(fn `UserConstructionScript`)