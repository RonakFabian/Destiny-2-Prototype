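; BP_MissionEnemyHolder is a mission actor that triggers the next mission event once every enemy in its list has died.
; On BeginPlay it binds to each listed enemy's death delegate, or prints a warning naming itself if the list is empty.
; Each death removes that enemy from the list, and emptying the list calls ExecuteNextMissionEvent.
; Debug prints remain, and EnemyCount is set but not read.
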(event `self.ReceiveBeginPlay`
  (bind _enemylist (`self.EnemyList`))
  (bind _returnvalue (`KismetArrayLibrary.Array_Length` _enemylist))
  (if (== _returnvalue 0)
    (`KismetSystemLibrary.PrintString` (`KismetStringLibrary.Concat_StrStr` "No enemy references in " (`KismetSystemLibrary.GetDisplayName` self)))
    (else
      (set `self.enemyCount` (+ _returnvalue 1))
      (for _array_element _enemylist
        (add `/Game/Blueprints/Enemy.OnEnemyDeath` _array_element (delegate `OnEnemyDeathEvent`)))
      (for _array_element_2 _enemylist
        (`KismetSystemLibrary.PrintString` (`KismetSystemLibrary.GetDisplayName` _array_element_2))))))

(event `OnEnemyDeathEvent`
  (params (`Enemy Type` :type "/Game/Quest/FEnemyType Enum" :default "NewEnumerator0") (DeadEnemy :type "Actor Object Reference"))
  (bind _enemylist (`self.EnemyList`))
  (bind _asenemy (cast `/Game/Blueprints/Enemy` DeadEnemy))
  (`KismetArrayLibrary.Array_RemoveItem` _enemylist _asenemy)
  (`KismetSystemLibrary.PrintString` "Hello")
  (if (== (`KismetArrayLibrary.Array_Length` _enemylist) 0)
    (`/Game/Quest/MissionEventHelper.ExecuteNextMissionEvent`)))

(fn `UserConstructionScript`
  (`parent.UserConstructionScript`))